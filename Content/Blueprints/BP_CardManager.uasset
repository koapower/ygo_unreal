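; Card manager that holds the card database, per-player decks and hands, and card instances for a card game.
; It loads card data from a DataTable keyed by integer row name and shuffles each deck on initialization.
; Drawing and deck searches create ID-numbered card instances, with draws stored in hands by instance ID.
; BP_Card actors spawn separately through a pool that hides and reuses destroyed cards.
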(event EventBeginPlay)

(event Collision|EventActorBeginOverlap
  (params (OtherActor :type Actor%20Object%20Reference)))

(event EventTick
  (params (DeltaSeconds :type Float%20%28single-precision%29)))

(fn ConstructionScript)

(fn LoadCardDatabase
  (params (CardDataTable :type Data%20Table%20Object%20Reference))
  (bind _carddatabase (Variables|Default|GetCardDatabase))
  (Utilities|IsValid CardDataTable
    (:Is%20Valid
      (Utilities|Map|Clear _carddatabase)
      (bind _outrownames (DataTable|GetDataTableRowNames CardDataTable))
      (for _array_element _outrownames
        (bind _returnvalue (Utilities|GetDataTableRow CardDataTable _array_element)
          (:then
            (Utilities|Map|Add _carddatabase (Math|Conversions|ToInteger(Byte) (Utilities|String|ToString(Name) _array_element)) _returnvalue)))))
    (:Is%20Not%20Valid
      (Development|PrintText "card data table is null! Failed to load card database!"))))

(fn InitializePlayerDeck
  (params (PlayerController :type BP%20YGO%20Player%20Controller%20Object%20Reference) (DeckData :type STR%20Deck%20Data%20Structure))
  (Utilities|IsValid PlayerController
    (:Is%20Valid
      (Utilities|Array|Shuffle (.mainDeck (Utilities|Struct|BreakSTR_DeckData DeckData)))
      (Utilities|Map|Add (Variables|Default|GetPlayerDecks) PlayerController DeckData)
      (Utilities|Map|Add (Variables|Default|GetPlayerHands) PlayerController (Utilities|Struct|MakeSTR_HandCardData (LocalVariables|GetemptyHandCards))))
    (:Is%20Not%20Valid
      (Development|PrintText "PlayerController is null! Failed to initialize player deck"))))

(fn SpawnCard
  (params (CardId :type Integer) (OwnerController :type BP%20YGO%20Player%20Controller%20Object%20Reference) (SpawnLocation :type Vector))
  (if (.ReturnValue (Utilities|Map|Find (Variables|Default|GetCardDatabase) CardId))
    (bind _newcard (CallFunction|GetorCreateCardActor))
    (Transformation|SetActorLocation _newcard SpawnLocation false true)
    (Default|InitializeCard _newcard CardId OwnerController)
    (return _newcard)
    (else
      (Development|PrintText (Utilities|Text|FormatText "Failed to find card data of id {0} in card database!" CardId))
      (return 0))))

(fn DestroyCard
  (params (card :type BP%20Card%20Object%20Reference))
  (Utilities|IsValid card
    (:Is%20Valid
      (CallFunction|RecycleCardActor card))))

(fn DrawCards
  (params (PlayerController :type BP%20YGO%20Player%20Controller%20Object%20Reference) (Count :type Integer))
  (bind _playerdecks (Variables|Default|GetPlayerDecks))
  (bind _playerhands (Variables|Default|GetPlayerHands))
  (bind (_value _returnvalue) (Utilities|Map|Find _playerdecks PlayerController))
  (bind (_value_2 _returnvalue_2) (Utilities|Map|Find _playerhands PlayerController))
  (Utilities|IsValid PlayerController
    (:Is%20Valid
      (if (and _returnvalue _returnvalue_2)
        (LocalVariables|Setdeck (.mainDeck (Utilities|Struct|BreakSTR_DeckData _value)))
        (LocalVariables|Sethand (Utilities|Struct|BreakSTR_HandCardData _value_2))
        (Utilities|FlowControl|ForLoopwithBreak 1 Count :!label _label
          (:LoopBody
            (if (== (Utilities|Array|Length (LocalVariables|Getdeck)) 0)
              (goto _label Break)
              (else
                (Utilities|Array|RemoveIndex (LocalVariables|Getdeck))
                (bind _instanceid (CallFunction|CreateCardInstance (Utilities|Array|Get(acopy) (LocalVariables|Getdeck)) PlayerController))
                ;[0.15 0.15 0.15 0.5] They contain instanceId, not cardId
                (Utilities|Array|Add (LocalVariables|Gethand) _instanceid)
                (Utilities|Array|Add (LocalVariables|GetdrawnCards) 0))))
          (:Completed
            (return (LocalVariables|GetdrawnCards))))
        (else
          (return (LocalVariables|GetdrawnCards)))))
    (:Is%20Not%20Valid
      (return (LocalVariables|GetdrawnCards)))))

(fn SearchDeck
  (params (PlayerController :type BP%20YGO%20Player%20Controller%20Object%20Reference) (CardId :type Integer))
  (bind _playerdecks (Variables|Default|GetPlayerDecks))
  (bind (_value _returnvalue) (Utilities|Map|Find _playerdecks PlayerController))
  (bind _maindeck (Utilities|Struct|BreakSTR_DeckData _value))
  (bind _returnvalue_2 (Utilities|Array|FindItem _maindeck CardId))
  (Utilities|IsValid PlayerController
    (:Is%20Valid
      (if _returnvalue
        (if (>= _returnvalue_2 0)
          (Utilities|Array|RemoveIndex _maindeck _returnvalue_2)
          (bind _instanceid (CallFunction|CreateCardInstance CardId PlayerController))
          (return _instanceid)
          (else
            (return -1)))
        (else
          (return -1))))
    (:Is%20Not%20Valid
      (return -1))))

(fn ShuffleDeck
  (params (PlayerController :type BP%20YGO%20Player%20Controller%20Object%20Reference))
  (bind _playerdecks (Variables|Default|GetPlayerDecks))
  (bind (_value _returnvalue) (Utilities|Map|Find _playerdecks PlayerController))
  (Utilities|IsValid PlayerController
    (:Is%20Valid
      (if _returnvalue
        (Utilities|Array|Shuffle (.mainDeck (Utilities|Struct|BreakSTR_DeckData _value)))
        (else
          (Development|PrintText (Utilities|Text|FormatText "Failed to find deck for playerController")))))
    (:Is%20Not%20Valid
      (Development|PrintText "playercontroller is null! failed to shuffledeck"))))

(fn GetCardData
  (params (CardId :type Integer))
  (bind _carddatabase (Variables|Default|GetCardDatabase))
  (bind (_value _returnvalue) (Utilities|Map|Find _carddatabase CardId))
  (return _value _returnvalue))

(fn GetCardInstance
  (params (InstanceId :type Integer))
  (bind _cardinstances (Variables|Default|GetCardInstances))
  (bind (_value _returnvalue) (Utilities|Map|Find _cardinstances InstanceId))
  (return _value _returnvalue))

(fn GetHandCount
  (params (PlayerController :type BP%20YGO%20Player%20Controller%20Object%20Reference))
  (bind _playerhands (Variables|Default|GetPlayerHands))
  (bind (_value _returnvalue) (Utilities|Map|Find _playerhands PlayerController))
  (if _returnvalue
    (return (Utilities|Array|Length (Utilities|Struct|BreakSTR_HandCardData _value)))
    (else
      (return 0))))

(fn GetDeckCount
  (params (PlayerController :type BP%20YGO%20Player%20Controller%20Object%20Reference))
  (bind _playerdecks (Variables|Default|GetPlayerDecks))
  (bind (_value _returnvalue) (Utilities|Map|Find _playerdecks PlayerController))
  (if _returnvalue
    (return (Utilities|Array|Length (.mainDeck (Utilities|Struct|BreakSTR_DeckData _value))))
    (else
      (return 0))))

(fn CreateCardInstance
  (params (CardId :type Integer) (OwnerController :type BP%20YGO%20Player%20Controller%20Object%20Reference))
  (bind _carddatabase (Variables|Default|GetCardDatabase))
  (bind _nextinstanceid (Variables|Default|GetNextInstanceId))
  (bind (_value _returnvalue) (Utilities|Map|Find _carddatabase CardId))
  (bind _str_cardinstance (Utilities|Struct|MakeSTR_CardInstance _value _nextinstanceid OwnerController 0))
  (bind _instanceid (Utilities|Struct|BreakSTR_CardInstance _str_cardinstance))
  (if _returnvalue
    (Math|Integer|IncrementInt _nextinstanceid
      (:%20%20
        (Utilities|Map|Add (Variables|Default|GetCardInstances) _instanceid _str_cardinstance)
        (return _instanceid)))
    (else
      (return -1))))

(fn GetorCreateCardActor
  (bind _cardpool (Variables|Default|GetCardPool))
  (bind _returnvalue (Utilities|Array|Length _cardpool))
  (bind _returnvalue_2 (- _returnvalue 1))
  (bind _output (Utilities|Array|Get(acopy) _cardpool _returnvalue_2))
  (if (> _returnvalue 0)
    (Utilities|Array|RemoveIndex _cardpool _returnvalue_2)
    (Rendering|SetActorHiddenInGame _output false)
    (return _output)
    (else
      (bind _returnvalue_3 (Game|SpawnActorfromClass "/Game/Blueprints/BP_Card.BP_Card_C" (Math|Transform|MakeTransform "0, 0, 0") "AlwaysSpawn" "MultiplyWithRoot" 0 0))
      (return _returnvalue_3))))

(fn RecycleCardActor
  (params (Card :type BP%20Card%20Object%20Reference))
  (Utilities|IsValid Card
    (:Is%20Valid
      (Rendering|SetActorHiddenInGame Card true)
      ;[0.15 0.15 0.15 0.5] so far away
      (Transformation|SetActorLocation Card "0.000000,0.000000,-1000.000000" false false)
      (Utilities|Array|Add (Variables|Default|GetCardPool) Card))))