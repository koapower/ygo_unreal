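; Player controller for a YGO card duel that creates the local debug HUD and points the view at the player's side of the field.
; On BeginPlay it binds to the game mode's OnDuelStarted, which triggers SetCamera for the local controller.
; SetCamera reads the player ID from player state index 0 and selects a tagged CameraActor.
; The P key prints the player's ID, life points and hand count.
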(event Custom|On%20Duel%20Started
  (if (Pawn|IsLocalPlayerController)
    (CallFunction|SetCamera)
    (Development|PrintText "on all players ready")))

(event EventBeginPlay
  (if (Pawn|IsLocalPlayerController)
    (bind _returnvalue (UserInterface|CreateWidget "/Game/UI/WBP_YGODebugHUD.WBP_YGODebugHUD_C" self))
    (UserInterface|Viewport|AddtoViewport _returnvalue 0)
    (bind _asbp_ygogame_mode_cppver (Utilities|Casting|CastToBP_YGOGameMode_CPPVER (Game|GetGameMode)))
    (EventDispatchers|BindEventtoOnDuelStarted _asbp_ygogame_mode_cppver (delegate Custom|On%20Duel%20Started))))

(event EventTick
  (params (DeltaSeconds :type Float%20%28single-precision%29)))

(event Input|KeyboardEvents|P
  (params (Key :type Key%20Structure :default "None"))
  (:Pressed
    (bind _asygoplayer_state (Utilities|Casting|CastToYGOPlayerState (Variables|Default|GetPlayerState)))
    (Development|PrintText (Utilities|Text|FormatText "Player {0}, LP: {1}, Hand: {2}" (Variables|/Script/YGO_unreal.YGOPlayerState|GetYGOPlayerID _asygoplayer_state) (Variables|/Script/YGO_unreal.YGOPlayerState|GetLifePoints _asygoplayer_state) (Variables|/Script/YGO_unreal.YGOPlayerState|GetHandCount _asygoplayer_state)))))

(fn ConstructionScript)

(fn SetCamera
  (bind _asbp_ygoplayer_state_cppver (Utilities|Casting|CastToBP_YGOPlayerState_CPPVER (Game|GetPlayerState 0)))
  ;[0.15 0.15 0.15 0.5] 0 is blue, not 0 is red
  (if (== (Variables|/Script/YGO_unreal.YGOPlayerState|GetYGOPlayerID _asbp_ygoplayer_state_cppver) 0)
    (LocalVariables|SetcamTagName "cameraS")
    (else
      (LocalVariables|SetcamTagName "cameraO")))
  (bind _outactors (Actor|GetAllActorsOfClasswithTag "/Script/Engine.CameraActor" (LocalVariables|GetcamTagName)))
  (Utilities|IsValid (Utilities|Array|Get(acopy) _outactors)
    (:Is%20Valid
      (Game|Player|SetViewTargetwithBlend (Utilities|Array|Get(acopy) _outactors) 0.0 "VTBlend_Linear" 0.0 false)
      (Development|PrintText (Utilities|Text|FormatText "set camera {0}, playerid {1}" (LocalVariables|GetcamTagName) (Variables|/Script/YGO_unreal.YGOPlayerState|GetYGOPlayerID _asbp_ygoplayer_state_cppver))))
    (:Is%20Not%20Valid
      (Development|PrintText (Utilities|Text|FormatText "Failed to find camera with tag {0}" (LocalVariables|GetcamTagName))))))