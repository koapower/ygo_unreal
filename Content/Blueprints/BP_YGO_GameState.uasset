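; Game state for a two-player card game (YGO) that tracks the game-start phase and spawns cards onto the field.
; Multicast_GameStarted sets the server-started phase; Tick then waits for two entries in PlayerArray before switching to the client-started phase and calling CallOnGameStarted.
; SpawnCard runs only with authority, using FieldManager to create a face-down card owned by the game state and move it to a position chosen by player index.
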(event Custom|Multicast_GameStarted
  (Variables|Default|SetcurrentPhase "NewEnumerator1")
  (Development|PrintString "set phase: on server game started"))

(event EventBeginPlay)

(event EventTick
  (params (DeltaSeconds :type Float%20%28single-precision%29))
  (switch Utilities|FlowControl|Switch|SwitchonE_GameStatePhase (Variables|Default|GetcurrentPhase)
    (:NewEnumerator1
      (if (== 2 (Utilities|Array|Length (Variables|Default|GetPlayerArray)))
        (Variables|Default|SetcurrentPhase "NewEnumerator2")
        (Development|PrintString "set phase: on client game started")
        (Default|CallOnGameStarted)))))

(fn ConstructionScript)

(fn SpawnCard
  (params (playerIndex :type Integer))
  (bind _fieldmanager (Variables|Default|GetFieldManager))
  (if (Ability|HasAuthority)
    (bind _cardobject (Default|SpawnCard _fieldmanager -1))
    (Actor|SetOwner _cardobject self)
    (Variables|/Game/Blueprints/BP_Card.BP_Card_C|SetisFacingDown _cardobject true)
    (if (== playerIndex 0)
      (LocalVariables|SetfieldPos "NewEnumerator0")
      (else
        (LocalVariables|SetfieldPos "NewEnumerator15")))
    (Default|MoveCardtoPos _fieldmanager _cardobject (LocalVariables|GetfieldPos))))