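; Server game mode for a two-player Yu-Gi-Oh!-style card game, handling match start and player actions.
; It sets up field, card and turn managers, then delegates validated summon, set and draw requests to them.
; Two start flows coexist: login-triggered StartGame using managers, and ready-triggered OnStartGame using its own deck and hand maps.
; Attack, phase advance, position change, battle, card movement, win checks and opponent lookup are stubs.
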(event Custom|OnPlayerReady
  (bind _result (Math|Integer|IncrementInt (Variables|Default|GetPlayersReadyCount))
    (:%20%20
      (if (== _result 2)
        (CallFunction|OnStartGame)))))

(event Custom|OnStartGame
  (bind _returnvalue (Game|GetGameState))
  (bind _playerarray (Variables|/Script/Engine.GameStateBase|GetPlayerArray _returnvalue))
  (Development|PrintText "Server OnStartGame")
  (for (_array_element _array_index) _playerarray
    (bind _asbp_ygo_player_state (Utilities|Casting|CastToBP_YGO_PlayerState _array_element))
    (CallFunction|InitializePlayer _asbp_ygo_player_state _array_index))
  (bind _asbp_ygo_player_state_2 (Utilities|Casting|CastToBP_YGO_PlayerState (.OutItem (Utilities|Array|Random _playerarray))))
  (Variables|Default|SetTurnPlayer _asbp_ygo_player_state_2)
  (bind _asbp_ygo_game_state (Utilities|Casting|CastToBP_YGO_GameState (Game|GetGameState)))
  (Default|MulticastGameStarted _asbp_ygo_game_state))

(event EventBeginPlay
  (CallFunction|InitializeManagers))

(event EventTick
  (params (DeltaSeconds :type Float%20%28single-precision%29)))

(event EventPostLogin
  (params (NewPlayer :type Player%20Controller%20Object%20Reference))
  (bind _playerlist (Variables|Game|GetPlayerList))
  (bind _asbp_ygo_player_controller (Utilities|Casting|CastToBP_YGO_PlayerController NewPlayer))
  (bind _returnvalue (Utilities|Array|Add _playerlist _asbp_ygo_player_controller))
  (Development|PrintText (Utilities|Text|FormatText "Player {0} joined" (+ _returnvalue 1)))
  (if (== (Utilities|Array|Length _playerlist) 2)
    (Game|StartGame)))

(event Custom|ServerDrawCards
  (params (PlayerController :type BP%20YGO%20Player%20Controller%20Object%20Reference) (Count :type Integer))
  (Actions|ProcessDrawCards PlayerController Count))

(event Custom|ServerSummon
  (params (PlayerController :type BP%20YGO%20Player%20Controller%20Object%20Reference) (CardInstanceId :type Integer) (SummonType :type E_SummonType%20Enum :default "NewEnumerator0") (CardPosition :type E_CardPosition%20Enum :default "NewEnumerator0") (IsOnOwnField :type Boolean) (FieldPosition :type E_FieldPosition%20Enum :default "NewEnumerator30") (Tribute :type Array%20of%20Integers))
  (if IsOnOwnField
    (Actions|ProcessSummon PlayerController CardInstanceId SummonType CardPosition PlayerController FieldPosition Tribute)
    (else
      (bind _opponentplayer (CallFunction|GetOpponent PlayerController))
      (Actions|ProcessSummon PlayerController CardInstanceId SummonType CardPosition _opponentplayer FieldPosition))))

(event Custom|ServerSetCard
  (params (PlayerController :type BP%20YGO%20Player%20Controller%20Object%20Reference) (CardInstanceId :type Integer) (IsOnOwnField :type Boolean) (FieldPosition :type E_FieldPosition%20Enum :default "NewEnumerator30"))
  (if IsOnOwnField
    (Actions|ProcessSetCard PlayerController CardInstanceId PlayerController FieldPosition)
    (else
      (bind _opponentplayer (CallFunction|GetOpponent PlayerController))
      (Actions|ProcessSetCard PlayerController CardInstanceId _opponentplayer FieldPosition))))

(event Custom|ServerAttack
  (params (PlayerController :type BP%20YGO%20Player%20Controller%20Object%20Reference) (AttackerInstanceId :type Integer) (TargetInstanceId :type Integer))
  (Actions|ProcessAttack PlayerController AttackerInstanceId TargetInstanceId))

(event Custom|ServerNextPhase
  (params (NextPhase :type E_TurnPhase%20Enum :default "NewEnumerator0"))
  (Actions|AdvancePhase NextPhase))

(event Custom|ServerChangeCardPosition
  (params (PlayerController :type BP%20YGO%20Player%20Controller%20Object%20Reference) (InstanceId :type Integer) (NewCardPosition :type E_CardPosition%20Enum :default "NewEnumerator0"))
  (Actions|ProcessChangeCardPosition PlayerController InstanceId NewCardPosition))

(event Custom|OnGameStarted)

(event Custom|OnGameEnded
  (params (Winner :type BP%20YGO%20Player%20State%20Object%20Reference) (Reason :type String)))

(fn ConstructionScript)

(fn InitializePlayer
  (params (PlayerState :type BP%20YGO%20Player%20State%20Object%20Reference) (index :type Integer))
  (bind _decktable (Variables|Data|GetDeckTable))
  (bind _deck (LocalVariables|Getdeck))
  (bind _decklist (Variables|Default|GetDeckList))
  (bind _handcardlist (Variables|Default|GetHandCardList))
  (bind _maindeck (Utilities|Struct|BreakSTR_DeckData _deck))
  (Variables|/Game/Blueprints/BP_YGO_PlayerState.BP_YGO_PlayerState_C|SetPlayerIndex PlayerState index)
  ;[0.15 0.15 0.15 0.5] Set LP
  (Variables|/Game/Blueprints/BP_YGO_PlayerState.BP_YGO_PlayerState_C|SetLP PlayerState (Variables|Rules|GetStartLP))
  ;[0.15 0.15 0.15 0.5] Setup main deck, store it inside DeckList
  (bind _outrownames (DataTable|GetDataTableRowNames _decktable))
  (for _array_element _outrownames
    (bind _returnvalue (Utilities|GetDataTableRow _decktable _array_element)
      (:then
        (Utilities|Array|Add _maindeck (Utilities|Struct|BreakSTR_DeckRow _returnvalue)))))
  (Utilities|Array|Shuffle _maindeck)
  (Utilities|Map|Remove _decklist PlayerState)
  (Utilities|Map|Add _decklist PlayerState _deck)
  ;[0.15 0.15 0.15 0.5] Set Deck card count
  (Variables|/Game/Blueprints/BP_YGO_PlayerState.BP_YGO_PlayerState_C|SetDeckCardCount PlayerState (Utilities|Array|Length _maindeck))
  ;[0.15 0.15 0.15 0.5] Draw Initial hand
  (Utilities|Map|Remove _handcardlist PlayerState)
  (Utilities|Map|Add _handcardlist PlayerState (LocalVariables|Gethandcard))
  (CallFunction|DrawCard PlayerState (Variables|Rules|GetInitialHandSize)))

(fn DrawCard
  (params (PlayerState :type BP%20YGO%20Player%20State%20Object%20Reference) (Count :type Integer))
  (bind (_deckdata _issuccessful) (CallFunction|GetPlayerDeckData PlayerState))
  (if _issuccessful
    (bind (_handcarddata _issuccessful_2) (CallFunction|GetPlayerHandCardData PlayerState))
    (if _issuccessful_2
      ;[0.15 0.15 0.15 0.5] draw cards to local var drawCards
      (for _index (range 1 Count)
        (Utilities|Array|Add (LocalVariables|GetdrawCards) (Utilities|Array|Get(acopy) (.mainDeck (Utilities|Struct|BreakSTR_DeckData _deckdata))))
        (Utilities|Array|RemoveIndex (.mainDeck (Utilities|Struct|BreakSTR_DeckData _deckdata))))
      ;[0.15 0.15 0.15 0.5] add count to hand card count
      (Variables|/Game/Blueprints/BP_YGO_PlayerState.BP_YGO_PlayerState_C|SetHandCardCount PlayerState (+ (Variables|/Game/Blueprints/BP_YGO_PlayerState.BP_YGO_PlayerState_C|GetHandCardCount PlayerState) Count))
      ;[0.15 0.15 0.15 0.5] minus count to deck card count
      (Variables|/Game/Blueprints/BP_YGO_PlayerState.BP_YGO_PlayerState_C|SetDeckCardCount PlayerState (- (Variables|/Game/Blueprints/BP_YGO_PlayerState.BP_YGO_PlayerState_C|GetDeckCardCount PlayerState) Count))
      ;[0.15 0.15 0.15 0.5] Add cards to hand (server)
      (for _array_element (LocalVariables|GetdrawCards)
        (Utilities|Array|Add (Utilities|Struct|BreakSTR_HandCardData _handcarddata) _array_element))
      ;[0.15 0.15 0.15 0.5] Call add cards to hand (for certain player)
      (bind _asbp_ygo_player_controller (Utilities|Casting|CastToBP_YGO_PlayerController (Game|GetPlayerController PlayerState)))
      (Default|ClientAddCardstoHand _asbp_ygo_player_controller (LocalVariables|GetdrawCards)))))

(fn GetPlayerDeckData
  (params (playerState :type BP%20YGO%20Player%20State%20Object%20Reference))
  (bind _decklist (Variables|Default|GetDeckList))
  (bind (_value _returnvalue) (Utilities|Map|Find _decklist playerState))
  (if _returnvalue
    (return _value _returnvalue)
    (else
      (Development|PrintString "Failed to find deck for player!")
      (return "" _returnvalue))))

(fn GetPlayerHandCardData
  (params (playerState :type BP%20YGO%20Player%20State%20Object%20Reference))
  (bind _handcardlist (Variables|Default|GetHandCardList))
  (bind (_value _returnvalue) (Utilities|Map|Find _handcardlist playerState))
  (if _returnvalue
    (return _value _returnvalue)
    (else
      (Development|PrintString "Failed to find handcard for player!")
      (return "" _returnvalue))))

(fn StartGame
  (bind _playerlist_copy (LocalVariables|GetPlayerList_copy))
  (bind _playerlist (Variables|Game|GetPlayerList))
  ;[0.15 0.15 0.15 0.5] Check players are valid
  (bind _array_element (Utilities|Array|ForEachLoopwithBreak (Variables|Game|GetPlayerList))
    (:LoopBody
      (Utilities|IsValid _array_element
        (:Is%20Not%20Valid
          (Development|PrintText "Cannot start game: missing player")
          (return))))
    (:Completed
      (Variables|Game|SetCurrentGameProgressState "NewEnumerator1")
      (for _array_element_2 (Variables|Game|GetPlayerList)
        (Default|InitializePlayer _array_element_2 (Variables|Rules|GetStartLP))
        (for _array_element_3 (Variables|Game|GetPlayerList)
          (Utilities|Array|Add _playerlist_copy _array_element_3))
        (Default|InitializeField (Variables|Manager|GetFieldManager) _playerlist_copy)
        (Default|InitializeTurn (Variables|Manager|GetTurnManager) _playerlist (.OutItem (Utilities|Array|Random _playerlist)))
        (CallFunction|InitializePlayerDecks)
        (CallFunction|InitialDraw)
        (Variables|Game|SetCurrentGameProgressState "NewEnumerator2")
        (Default|StartGame (Variables|Manager|GetTurnManager))
        (CallFunction|OnGameStarted)
        (Development|PrintText "Game started!")))))

(fn EndGame
  (params (Winner :type BP%20YGO%20Player%20Controller%20Object%20Reference) (Reason :type String))
  (Variables|Game|SetCurrentGameProgressState "NewEnumerator3")
  (bind _asbp_ygo_player_state (Utilities|Casting|CastToBP_YGO_PlayerState (Variables|/Script/Engine.Controller|GetPlayerState Winner)))
  (CallFunction|OnGameEnded _asbp_ygo_player_state Reason)
  (Utilities|IsValid Winner
    (:Is%20Valid
      (LocalVariables|SetwinnerName (Utilities|GetDisplayName Winner)))
    (:Is%20Not%20Valid
      (LocalVariables|SetwinnerName (Utilities|String|MakeLiteralString "Draw"))))
  (Development|PrintText (Utilities|Text|FormatText "Game ended! Winner: {0}, Reason: {1}" (LocalVariables|GetwinnerName) Reason)))

(fn GetFieldManager
  (return (Variables|Manager|GetFieldManager)))

(fn GetTurnManager
  (return (Variables|Manager|GetTurnManager)))

(fn GetCardManager
  (return (Variables|Manager|GetCardManager)))

(fn ProcessDrawCards
  (params (PlayerController :type BP%20YGO%20Player%20Controller%20Object%20Reference) (Count :type Integer))
  (bind _returnvalue (Utilities|IsValid PlayerController))
  (bind _cardmanager (Variables|Manager|GetCardManager))
  (bind _cardmanager_2 (Variables|Manager|GetCardManager))
  (bind _returnvalue_2 (Utilities|IsValid _cardmanager))
  (if (and _returnvalue_2 _returnvalue)
    (bind _deckremaincount (Default|GetDeckCount _cardmanager_2 PlayerController))
    (LocalVariables|SetplayerNoCardToDraw (> Count _deckremaincount))
    (bind _drawcards (Default|DrawCards _cardmanager_2 PlayerController Count))
    (if (LocalVariables|GetplayerNoCardToDraw)
      (bind _opponentplayer (CallFunction|GetOpponent PlayerController))
      (Game|EndGame _opponentplayer (Utilities|GetDisplayName PlayerController))
      (return false)
      (else
        (Default|ClientRecieveCards PlayerController _drawcards)
        (return true)))
    (else
      (Development|PrintText (Utilities|Text|FormatText "Failed to process draw cards. Player valid {0}, cardmanager valid {1}" _returnvalue _returnvalue_2))
      (return false))))

(fn ProcessSummon
  (params (PlayerController :type BP%20YGO%20Player%20Controller%20Object%20Reference) (CardInstanceId :type Integer) (SummonType :type E_SummonType%20Enum :default "NewEnumerator0") (CardPosition :type E_CardPosition%20Enum :default "NewEnumerator0") (FieldOwner :type BP%20YGO%20Player%20Controller%20Object%20Reference) (FieldPosition :type E_FieldPosition%20Enum :default "NewEnumerator30") (Tribute :type Array%20of%20Integers))
  (bind _returnvalue (Utilities|IsValid PlayerController))
  (bind _returnvalue_2 (Utilities|Enum|Equal(Enum) SummonType "NewEnumerator1"))
  (bind _returnvalue_3 (Utilities|Enum|Equal(Enum) SummonType "NewEnumerator2"))
  (bind _fieldmanager (Variables|Manager|GetFieldManager))
  (bind _turnmanager (Variables|Manager|GetTurnManager))
  (bind _removecards (LocalVariables|Getremovecards))
  (bind _cardmanager (Variables|Manager|GetCardManager))
  (bind _returnvalue_4 (Utilities|IsValid _fieldmanager))
  (bind _returnvalue_5 (Utilities|IsValid _turnmanager))
  (bind _returnvalue_6 (Utilities|IsValid _cardmanager))
  (bind _returnvalue_7 (or _returnvalue_2 _returnvalue_3))
  (if (Math|Boolean|ANDBoolean _returnvalue _returnvalue_4 _returnvalue_5 _returnvalue_6)
    (bind _yesno (Default|IsPlayerTurn (Variables|Manager|GetTurnManager) PlayerController))
    (if _yesno
      ;[0.15 0.15 0.15 0.5] if isNormalSummon
      (if _returnvalue_7
        (bind _can (Default|CanNormalSummon (Variables|Manager|GetTurnManager)))
        (if _can
          _
          (else
            (Default|ClientActionFailed PlayerController "Cannot normal summon")
            (return false))))
      (bind (_cardinstance _found) (Default|GetCardInstance (Variables|Manager|GetCardManager) CardInstanceId))
      (if _found
        (for _array_element Tribute
          (bind (_cardinstance_2 _found_2) (Default|GetCardInstance (Variables|Manager|GetCardManager)))
          (if _found_2
            (Utilities|Array|Add (LocalVariables|GetTributeCards) _cardinstance_2)
            (else
              (Default|ClientActionFailed PlayerController "Tribute Card not found")
              (return false))))
        ;[0.15 0.15 0.15 0.5] isMonsterCard
        (if (== (.cardType (Utilities|Struct|BreakSTR_CardData (.cardData (Utilities|Struct|BreakSTR_CardInstance _cardinstance)))) 0)
          ;[0.15 0.15 0.15 0.5] Check is position  available
          (bind _posobject (Default|GetPositionObject (Variables|Manager|GetFieldManager) FieldOwner FieldPosition))
          (bind _allcards (Default|GetAllCards _posobject))
          (if (Utilities|Array|IsEmpty _allcards)
            ;[0.15 0.15 0.15 0.5] Move tributes to gy
            (for _array_element_2 (LocalVariables|GetTributeCards) :!label _label
              (Rules|MoveCardto (.cardActor (Utilities|Struct|BreakSTR_CardInstance _array_element_2)) "NewEnumerator2"))
            ;[0.15 0.15 0.15 0.5] Summon card
            (bind _worldposition (Default|GetFieldPositionWorldLocation (Variables|Manager|GetFieldManager) FieldOwner FieldPosition))
            (bind _card (Default|SpawnCard (Variables|Manager|GetCardManager) (.cardId (Utilities|Struct|BreakSTR_CardData (.cardData (Utilities|Struct|BreakSTR_CardInstance _cardinstance)))) PlayerController _worldposition))
            (Utilities|IsValid _card
              (:Is%20Valid
                (Default|SetCardPosition _card CardPosition true)
                (Default|SetCardZone _card "NewEnumerator2")
                (Default|PlaceCard (Variables|Manager|GetFieldManager) _card FieldOwner FieldPosition CardPosition)
                (Utilities|Array|Add _removecards _card)
                (Default|RemoveCardsfromHand PlayerController _removecards)
                (if _returnvalue_7
                  (Default|ConsumeNormalSummon (Variables|Manager|GetTurnManager))
                  (Development|PrintText (Utilities|Text|FormatText "Player summoned cardid {0}" (.cardId (Utilities|Struct|BreakSTR_CardData (.cardData (Utilities|Struct|BreakSTR_CardInstance _cardinstance))))))
                  (return true)))
              (:Is%20Not%20Valid
                (Default|ClientActionFailed PlayerController "Failed to spawn card")
                (return false)))
            (else
              (LocalVariables|SetisTribute false)
              (bind _array_element_3 (Utilities|Array|ForEachLoopwithBreak (LocalVariables|GetTributeCards) :!label _label_2)
                (:LoopBody
                  (if (== (Utilities|Array|Get(acopy) _allcards) (.cardActor (Utilities|Struct|BreakSTR_CardInstance _array_element_3)))
                    (LocalVariables|SetisTribute true)
                    (goto _label_2 Break)))
                (:Completed
                  (if (LocalVariables|GetisTribute)
                    (goto _label)
                    (else
                      (Default|ClientActionFailed PlayerController "Position is occupied, cannot summon monster here")
                      (return false)))))))
          (else
            (Default|ClientActionFailed PlayerController "Card is not monster")
            (return false)))
        (else
          (Default|ClientActionFailed PlayerController "Card not found")
          (return false)))
      (else
        (Default|ClientActionFailed PlayerController "Not Your Turn")
        (return false)))
    (else
      (Development|PrintText (Utilities|Text|FormatText "Failed to process summon. validity: player {0}, fieldmanager {1}, turnmanager {2}, cardmanager {3}" _returnvalue _returnvalue_4 _returnvalue_5 _returnvalue_6))
      (return false))))

(fn ProcessSetCard
  (params (PlayerController :type BP%20YGO%20Player%20Controller%20Object%20Reference) (CardInstanceId :type Integer) (FieldOwner :type BP%20YGO%20Player%20Controller%20Object%20Reference) (FieldPosition :type E_FieldPosition%20Enum :default "NewEnumerator30"))
  (bind _removecards (LocalVariables|GetremoveCards))
  (if (Math|Boolean|ANDBoolean (Utilities|IsValid PlayerController) (Utilities|IsValid (Variables|Manager|GetFieldManager)) (Utilities|IsValid (Variables|Manager|GetTurnManager)) (Utilities|IsValid (Variables|Manager|GetCardManager)))
    (bind _yesno (Default|IsPlayerTurn (Variables|Manager|GetTurnManager) PlayerController))
    (if _yesno
      (bind (_cardinstance _found) (Default|GetCardInstance (Variables|Manager|GetCardManager) CardInstanceId))
      (if _found
        (switch int (.cardType (Utilities|Struct|BreakSTR_CardData (.cardData (Utilities|Struct|BreakSTR_CardInstance _cardinstance))))
          (:Default
            (LocalVariables|SetTargetZone "NewEnumerator3")
            (LocalVariables|SetCardPosition "NewEnumerator2"))
          (:0
            (LocalVariables|SetTargetZone "NewEnumerator2")
            (LocalVariables|SetCardPosition "NewEnumerator3")
            (bind _can (Default|CanNormalSummon (Variables|Manager|GetTurnManager)))
            (if _can
              _
              (else
                (Default|ClientActionFailed PlayerController "Cannot normal summon")
                (return false)))))
        (bind _isavailable (Default|IsPositionAvailable (Variables|Manager|GetFieldManager) FieldOwner FieldPosition))
        (if _isavailable
          (bind _worldposition (Default|GetFieldPositionWorldLocation (Variables|Manager|GetFieldManager) FieldOwner FieldPosition))
          (bind _card (Default|SpawnCard (Variables|Manager|GetCardManager) (.cardId (Utilities|Struct|BreakSTR_CardData (.cardData (Utilities|Struct|BreakSTR_CardInstance _cardinstance)))) PlayerController _worldposition))
          (Utilities|IsValid _card
            (:Is%20Valid
              (Default|SetCardPosition _card (LocalVariables|GetCardPosition) false)
              (Default|SetCardZone _card (LocalVariables|GetTargetZone))
              (Default|SetFaceUp _card false false)
              (Default|PlaceCard (Variables|Manager|GetFieldManager) _card FieldOwner FieldPosition (LocalVariables|GetCardPosition))
              (Utilities|Array|Add _removecards _card)
              (Default|RemoveCardsfromHand PlayerController _removecards)
              ;[0.15 0.15 0.15 0.5] is monster, set monster
              (if (== (.cardType (Utilities|Struct|BreakSTR_CardData (.cardData (Utilities|Struct|BreakSTR_CardInstance _cardinstance)))) 0)
                (Default|ConsumeNormalSummon (Variables|Manager|GetTurnManager))
                (Development|PrintText (Utilities|Text|FormatText "Player set card {0}" (.cardId (Utilities|Struct|BreakSTR_CardData (.cardData (Utilities|Struct|BreakSTR_CardInstance _cardinstance))))))
                (return true)))
            (:Is%20Not%20Valid
              (Default|ClientActionFailed PlayerController "Failed to spawn card")
              (return false)))
          (else
            (Default|ClientActionFailed PlayerController "Field position is occupied")
            (return false)))
        (else
          (Default|ClientActionFailed PlayerController "Card not found")
          (return false)))
      (else
        (Default|ClientActionFailed PlayerController "Not your turn")
        (return false)))
    (else
      (Development|PrintText "Something is null")
      (return false))))

(fn ProcessAttack
  (params (PlayerController :type BP%20YGO%20Player%20Controller%20Object%20Reference) (AttackerInstanceId :type Integer) (TargetInstanceId :type Integer))
  (if (not (and (Utilities|IsValid (Variables|Manager|GetTurnManager)) (Utilities|IsValid PlayerController)))
    (Development|PrintText "something is null")
    (return false)))

(fn AdvancePhase
  (params (NextTurnPhase :type E_TurnPhase%20Enum :default "NewEnumerator0"))
  (return false))

(fn CanNormalSummon
  (params (PlayerController :type BP%20YGO%20Player%20Controller%20Object%20Reference) (CardInstanceId :type Integer))
  (return false))

(fn CanAttack
  (params (AttackerInstanceId :type Integer) (TargetInstanceId :type Integer)))

(fn CheckWinConditions)

(fn CalculateBattle
  (params (Attacker :type %20Object%20Reference) (Target :type %20Object%20Reference)))

(fn DealBattleDamage
  (params (PlayerController :type BP%20YGO%20Player%20Controller%20Object%20Reference) (Damage :type Integer)))

(fn MoveCardto
  (params (Card :type BP%20Card%20Object%20Reference) (Destination :type E_FieldPosition%20Enum :default "NewEnumerator30")))

(fn GetGameProgressState
  (return (Variables|Game|GetCurrentGameProgressState)))

(fn GetPlayer1
  (return (Utilities|Array|Get(acopy) (Variables|Game|GetPlayerList))))

(fn GetPlayer2
  (return (Utilities|Array|Get(acopy) (Variables|Game|GetPlayerList) 1)))

(fn InitializeManagers
  (bind _returnvalue (Actor|GetActorOfClass "/Game/Blueprints/BP_FieldManager.BP_FieldManager_C"))
  (Variables|Manager|SetFieldManager _returnvalue)
  (bind _returnvalue_2 (Game|SpawnActorfromClass "/Game/Blueprints/BP_CardManager.BP_CardManager_C" (Math|Transform|MakeTransform "0, 0, 0") "Undefined" "MultiplyWithRoot" 0 0))
  (bind _output_get (Variables|Manager|SetCardManager _returnvalue_2))
  (Default|LoadCardDatabase _output_get (Variables|Data|GetCardDataTable))
  (bind _returnvalue_3 (Game|SpawnActorfromClass "/Game/Blueprints/BP_TurnManager.BP_TurnManager_C" (Math|Transform|MakeTransform "0, 0, 0") "Undefined" "MultiplyWithRoot" 0 0))
  (Variables|Manager|SetTurnManager _returnvalue_3))

(fn InitializePlayerDecks
  (bind _decktable (Variables|Data|GetDeckTable))
  (bind _outrownames (DataTable|GetDataTableRowNames _decktable))
  (for _array_element _outrownames
    (bind _returnvalue (Utilities|GetDataTableRow _decktable _array_element)
      (:then
        (Utilities|Array|Add (LocalVariables|GetDeck1) (Utilities|Struct|BreakSTR_DeckRow _returnvalue))
        (Utilities|Array|Add (LocalVariables|GetDeck2) (Utilities|Struct|BreakSTR_DeckRow _returnvalue)))))
  (Default|InitializePlayerDeck (Variables|Manager|GetCardManager) (Utilities|Array|Get(acopy) (Variables|Game|GetPlayerList)) (Utilities|Struct|MakeSTR_DeckData (LocalVariables|GetDeck1)))
  (Default|InitializePlayerDeck (Variables|Manager|GetCardManager) (Utilities|Array|Get(acopy) (Variables|Game|GetPlayerList) 1) (Utilities|Struct|MakeSTR_DeckData (LocalVariables|GetDeck2))))

(fn InitialDraw
  (for _array_element (Variables|Game|GetPlayerList)
    (Actions|ProcessDrawCards _array_element (Variables|Rules|GetInitialHandSize))))

(fn GetOpponent
  (params (Player :type BP%20YGO%20Player%20Controller%20Object%20Reference))
  (return 0))

(fn ProcessChangeCardPosition
  (params (PlayerController :type BP%20YGO%20Player%20Controller%20Object%20Reference) (InstanceId :type Integer) (CardPosition :type E_CardPosition%20Enum :default "NewEnumerator0"))
  (return false))