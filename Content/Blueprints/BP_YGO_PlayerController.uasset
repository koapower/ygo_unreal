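; Player controller for a two-player Yu-Gi-Oh-style card duel, handling local HUD, input, hand cards and Life Points stored on the PlayerState.
; Tick polls until both players exist, then binds game start, which picks a tagged camera by player index, and reports ready.
; Request functions convert cards to instance IDs and call server events that forward to the GameMode.
; Client feedback events, mouse handlers and OnHandChanged are empty stubs.
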(event Custom|Client_AddCardsToHand
  (params (cardId :type Array%20of%20Integers))
  (for _array_element cardId
    (Utilities|Array|Add (Variables|Default|GetHandCardIds) _array_element)))

(event Custom|Server_ReportReady
  (bind _asbp_ygo_game_mode (Utilities|Casting|CastToBP_YGO_GameMode (Game|GetGameMode)))
  (Default|OnPlayerReady _asbp_ygo_game_mode))

(event Custom|OnGameStarted
  (CallFunction|SetCamera)
  (Development|PrintText "Playercontroller ongamestarted complete"))

(event EventBeginPlay
  (bind _self self)
  (if (Pawn|IsLocalPlayerController)
    ;[0.15 0.15 0.15 0.5] HUD
    (bind _returnvalue (UserInterface|CreateWidget "/Game/UI/WBP_GameHUD.WBP_GameHUD_C" _self))
    (UserInterface|Viewport|AddtoViewport _returnvalue 0)
    (Input|AddMappingContext (PlayerController|LocalPlayerSubsystems|GetEnhancedInputLocalPlayerSubsystem _self) "/Game/Input/IMC_Player.IMC_Player" 0 "(bIgnoreAllPressedKeysUntilRelease=True,bForceImmediately=False,bNotifyUserSettings=False)")))

(event EventTick
  (params (DeltaSeconds :type Float%20%28single-precision%29))
  (if (Pawn|IsLocalPlayerController)
    ;[0.15 0.15 0.15 0.5] Wait until game state and player state are valid, bind events, report ready to server. After report, this will not be called anymore
    (if (not (Variables|Default|GetbHasBoundToGameEvents))
      (bind _isvalid (CallFunction|CheckIsGameStateValid))
      (if _isvalid
        (Variables|Default|SetbHasBoundToGameEvents true)
        (bind _asbp_ygo_game_state (Utilities|Casting|CastToBP_YGO_GameState (Game|GetGameState)))
        (EventDispatchers|BindEventtoOnGameStarted _asbp_ygo_game_state (delegate Custom|OnGameStarted))
        (Development|PrintText "On report to server player controller is ready")
        (CallFunction|ServerReportReady)))))

(event Custom|ServerDrawCards
  (params (Count :type Integer))
  (bind _gamemode (CallFunction|GetGameMode))
  (Default|ServerDrawCards _gamemode self Count))

(event Custom|ServerSummon
  (params (CardInstanceId :type Integer) (isNormalSummon :type Boolean) (CardPosition :type E_CardPosition%20Enum :default "NewEnumerator0") (FieldPosition :type E_FieldPosition%20Enum :default "NewEnumerator30"))
  (bind _gamemode (CallFunction|GetGameMode))
  (Default|ServerSummon _gamemode self CardInstanceId isNormalSummon CardPosition FieldPosition))

(event Custom|ServerSetCard
  (params (CardInstanceId :type Integer) (FieldPosition :type E_FieldPosition%20Enum :default "NewEnumerator30"))
  (bind _gamemode (CallFunction|GetGameMode))
  (Default|ServerSetCard _gamemode self CardInstanceId FieldPosition))

(event Custom|ServerAttack
  (params (AttackerInstanceId :type Integer) (TargetInstanceId :type Integer))
  (bind _gamemode (CallFunction|GetGameMode))
  (Default|ServerAttack _gamemode self AttackerInstanceId TargetInstanceId))

(event Custom|ServerNextPhase
  (params (NextPhase :type E_TurnPhase%20Enum :default "NewEnumerator0"))
  (bind _gamemode (CallFunction|GetGameMode))
  (Default|ServerNextPhase _gamemode NextPhase))

(event Custom|ServerChangeCardPosition
  (params (InstanceId :type Integer) (NewCardPosition :type E_CardPosition%20Enum :default "NewEnumerator0"))
  (bind _gamemode (CallFunction|GetGameMode))
  (Default|ServerChangeCardPosition _gamemode self InstanceId NewCardPosition))

(event Custom|ClientRecieveCards
  (params (CardInstanceIds :type Array%20of%20Integers)))

(event Custom|ClientActionFailed
  (params (Reason :type String)))

(event Custom|ClientPlayEffect
  (params (EffectName :type String)))

(event Custom|OnHandChanged)

(fn ConstructionScript
  (Variables|Default|SetbShowMouseCursor true)
  (Variables|Default|SetbEnableClickEvents true)
  (Variables|Default|SetbEnableMouseOverEvents true)
  (bind _asbp_ygo_player_state (Utilities|Casting|CastToBP_YGO_PlayerState (Variables|GetPlayerState)))
  (Variables|/Game/Blueprints/BP_YGO_PlayerState.BP_YGO_PlayerState_C|SetLP _asbp_ygo_player_state 8000)
  (Variables|/Game/Blueprints/BP_YGO_PlayerState.BP_YGO_PlayerState_C|SetCurrentAction _asbp_ygo_player_state "NewEnumerator0")
  (Input|SetInputModeGameandUI self 0 "DoNotLock" false false))

(fn CheckIsGameStateValid
  (bind _returnvalue (Game|GetGameState))
  (Utilities|IsValid _returnvalue
    (:Is%20Valid
      (Utilities|IsValid (Variables|GetPlayerState)
        (:Is%20Valid
          (bind _asbp_ygo_game_state (Utilities|Casting|CastToBP_YGO_GameState _returnvalue))
          (Development|PrintText (Utilities|Text|FormatText "gamestate.playerArray {0}/Expected 2" (Utilities|Array|Length (Variables|/Script/Engine.GameStateBase|GetPlayerArray _asbp_ygo_game_state))))
          (if (== 2 (Utilities|Array|Length (Variables|/Script/Engine.GameStateBase|GetPlayerArray _asbp_ygo_game_state)))
            (return true)))))))

(fn SetCamera
  (bind _asbp_ygo_player_state (Utilities|Casting|CastToBP_YGO_PlayerState (Variables|GetPlayerState)))
  ;[0.15 0.15 0.15 0.5] 0 is blue, not 0 is red
  (if (== (Variables|/Game/Blueprints/BP_YGO_PlayerState.BP_YGO_PlayerState_C|GetPlayerIndex _asbp_ygo_player_state) 0)
    (LocalVariables|SetcamTagName "cameraS")
    (else
      (LocalVariables|SetcamTagName "cameraO")))
  (bind _outactors (Actor|GetAllActorsOfClasswithTag "/Script/Engine.CameraActor" (LocalVariables|GetcamTagName)))
  (Utilities|IsValid (Utilities|Array|Get(acopy) _outactors)
    (:Is%20Valid
      (Game|Player|SetViewTargetwithBlend (Utilities|Array|Get(acopy) _outactors) 0.0 "VTBlend_Linear" 0.0 false))
    (:Is%20Not%20Valid
      (Development|PrintText (Utilities|Text|FormatText "Failed to find camera with tag {0}" (LocalVariables|GetcamTagName))))))

(fn InitializePlayer
  (params (StartingLifePoints :type Integer))
  (bind _asbp_ygo_player_state (Utilities|Casting|CastToBP_YGO_PlayerState (Variables|GetPlayerState)))
  (Variables|/Game/Blueprints/BP_YGO_PlayerState.BP_YGO_PlayerState_C|SetLP _asbp_ygo_player_state StartingLifePoints))

(fn GetLP
  (bind _asbp_ygo_player_state (Utilities|Casting|CastToBP_YGO_PlayerState (Variables|GetPlayerState)))
  (return (Variables|/Game/Blueprints/BP_YGO_PlayerState.BP_YGO_PlayerState_C|GetLP _asbp_ygo_player_state)))

(fn SetLP
  (params (NewLP :type Integer))
  (bind _asbp_ygo_player_state (Utilities|Casting|CastToBP_YGO_PlayerState (Variables|GetPlayerState)))
  (Variables|/Game/Blueprints/BP_YGO_PlayerState.BP_YGO_PlayerState_C|SetLP _asbp_ygo_player_state NewLP))

(fn TakeDamage
  (params (Damage :type Integer) (Type :type E_DamageType%20Enum :default "NewEnumerator0"))
  (bind _lp (Player|GetLP))
  (if (< (- _lp Damage) 0)
    (Player|SetLP (Class|KismetSystemLibrary|MakeLiteralInteger))
    (else
      (Player|SetLP (- _lp Damage)))))

(fn GainLP
  (params (Amount :type Integer))
  (bind _lp (Player|GetLP))
  (if (< (+ _lp Amount) 0)
    (Player|SetLP (Class|KismetSystemLibrary|MakeLiteralInteger))
    (else
      (Player|SetLP))))

(fn AddCardstoHand
  (params (cards :type Array%20of%20BP%20Card%20Object%20References))
  (for _array_element cards
    (Utilities|Array|Add (Variables|Default|GetHandCards) _array_element))
  (CallFunction|OnHandChanged))

(fn RemoveCardsfromHand
  (params (Cards :type Array%20of%20BP%20Card%20Object%20References))
  (for _array_element Cards
    (Utilities|Array|RemoveItem (Variables|Default|GetHandCards) _array_element))
  (CallFunction|OnHandChanged))

(fn GetHandCards
  (return (Variables|Default|GetHandCards)))

(fn GetHandCount
  (return (Utilities|Array|Length (Variables|Default|GetHandCards))))

(fn RequestDrawCards
  (params (Count :type Integer))
  (CallFunction|ServerDrawCards Count))

(fn RequestSummon
  (params (card :type BP%20Card%20Object%20Reference) (isNormalSummon :type Boolean) (CardPosition :type E_CardPosition%20Enum :default "NewEnumerator0") (FieldPosition :type E_FieldPosition%20Enum :default "NewEnumerator30"))
  (Utilities|IsValid card
    (:Is%20Valid
      (bind _instanceid (Default|GetInstanceId card))
      (CallFunction|ServerSummon _instanceid isNormalSummon CardPosition FieldPosition))
    (:Is%20Not%20Valid
      (Development|PrintText "RequestSummon but card is not valid!"))))

(fn RequestSetCard
  (params (Card :type BP%20Card%20Object%20Reference) (FieldPosition :type E_FieldPosition%20Enum :default "NewEnumerator30"))
  (Utilities|IsValid Card
    (:Is%20Valid
      (bind _instanceid (Default|GetInstanceId Card))
      (CallFunction|ServerSetCard _instanceid FieldPosition))
    (:Is%20Not%20Valid
      (Development|PrintText "RequestSetCard but card is not valid!"))))

(fn RequestChangeCardPosition
  (params (Card :type BP%20Card%20Object%20Reference) (NewCardPosition :type E_CardPosition%20Enum :default "NewEnumerator0"))
  (Utilities|IsValid Card
    (:Is%20Valid
      (bind _instanceid (Default|GetInstanceId Card))
      (CallFunction|ServerChangeCardPosition _instanceid NewCardPosition))
    (:Is%20Not%20Valid
      (Development|PrintText "RequestChangeCardPosition but card is not valid!"))))

(fn RequestAttack
  (params (AttackingCard :type BP%20Card%20Object%20Reference) (TargetCard :type BP%20Card%20Object%20Reference))
  (Utilities|IsValid AttackingCard
    (:Is%20Valid
      (bind _instanceid (Default|GetInstanceId AttackingCard))
      (Utilities|IsValid TargetCard
        (:Is%20Valid
          (bind _instanceid_2 (Default|GetInstanceId TargetCard))
          (CallFunction|ServerAttack _instanceid _instanceid_2))
        (:Is%20Not%20Valid
          (CallFunction|ServerAttack _instanceid (Class|KismetSystemLibrary|MakeLiteralInteger -1)))))
    (:Is%20Not%20Valid
      (Development|PrintText "RequestAttack but attack card is not valid!"))))

(fn RequestNextPhase
  (params (NextPhase :type E_TurnPhase%20Enum :default "NewEnumerator0"))
  (CallFunction|ServerNextPhase NextPhase))

(fn GetGameMode
  (bind _asbp_ygo_game_mode (Utilities|Casting|CastToBP_YGO_GameMode (Game|GetGameMode)))
  (return _asbp_ygo_game_mode))

(fn OnMouseClick)

(fn OnMouseHover)