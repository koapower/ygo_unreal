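; Turn manager for a two-player Yu-Gi-Oh!-style card game, running the phase sequence from Draw to End and alternating the turn player.
; It stores turn player, count, phase and battle step on BP_YGO_GameState, broadcasting turn and phase changes through multicast events.
; AdvancePhase enforces the order and skips battle on the first turn, while ForceSetPhase bypasses it.
; It also limits Normal Summons to Main Phases and a per-turn allowance.
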(event EventBeginPlay)

(event Collision|EventActorBeginOverlap
  (params (OtherActor :type Actor%20Object%20Reference)))

(event EventTick
  (params (DeltaSeconds :type Float%20%28single-precision%29)))

(event Custom|OnStanbyPhaseStart)

(event Custom|OnTurnChanged
  (params (NewTurnPlayer :type BP%20YGO%20Player%20State%20Object%20Reference) (TurnNumber :type Integer)))

(event Custom|OnMain2PhaseStart)

(event Custom|OnMain2PhaseEnd)

(event Custom|OnEndPhaseStart)

(event Custom|OnPhaseChanged
  (params (NewPhase :type E_TurnPhase%20Enum :default "NewEnumerator0") (OldPhase :type E_TurnPhase%20Enum :default "NewEnumerator0")))

(event Custom|OnDrawPhaseStart)

(event Custom|OnMain1PhaseStart)

(event Custom|OnMain1PhaseEnd)

(event Custom|OnBattlePhaseStart)

(event Custom|OnBattlePhaseEnd)

(fn ConstructionScript)

(fn InitializeTurn
  (params (Players :type Array%20of%20BP%20YGO%20Player%20Controller%20Object%20References) (StartingPlayer :type BP%20YGO%20Player%20Controller%20Object%20Reference))
  (Variables|Default|SetPlayers Players)
  (bind _asbp_ygo_player_state (Utilities|Casting|CastToBP_YGO_PlayerState (Variables|/Script/Engine.Controller|GetPlayerState StartingPlayer)))
  (bind _gamestate (CallFunction|GetGameState))
  (Variables|/Game/Blueprints/BP_YGO_GameState.BP_YGO_GameState_C|SetCurrentTurnPlayer _gamestate _asbp_ygo_player_state)
  (Variables|/Game/Blueprints/BP_YGO_GameState.BP_YGO_GameState_C|SetTurnCount _gamestate 0)
  (Variables|/Game/Blueprints/BP_YGO_GameState.BP_YGO_GameState_C|SetCurrentTurnPhase _gamestate "NewEnumerator0")
  (Variables|Default|SetisFirstTurn true))

(fn GetGameState
  (bind _asbp_ygo_game_state (Utilities|Casting|CastToBP_YGO_GameState (Game|GetGameState)))
  (return _asbp_ygo_game_state))

(fn EnterPhase
  (params (NextPhase :type E_TurnPhase%20Enum :default "NewEnumerator0"))
  (bind _gamestate (CallFunction|GetGameState))
  (bind _output_get (LocalVariables|SetOldPhase (Variables|/Game/Blueprints/BP_YGO_GameState.BP_YGO_GameState_C|GetCurrentTurnPhase _gamestate)))
  (bind _output_get_2 (Variables|/Game/Blueprints/BP_YGO_GameState.BP_YGO_GameState_C|SetCurrentTurnPhase _gamestate NextPhase))
  (CallFunction|OnPhaseChanged _output_get_2 _output_get)
  (CallFunction|BroadcastPhaseEvents _output_get_2))

(fn BroadcastPhaseEvents
  (params (Phase :type E_TurnPhase%20Enum :default "NewEnumerator0"))
  (switch Utilities|FlowControl|Switch|SwitchonE_TurnPhase Phase
    (:NewEnumerator0
      (CallFunction|OnDrawPhaseStart))
    (:NewEnumerator1
      (CallFunction|OnStanbyPhaseStart))
    (:NewEnumerator2
      (CallFunction|OnMain1PhaseStart))
    (:NewEnumerator3
      (CallFunction|OnBattlePhaseStart)
      (bind _gamestate (CallFunction|GetGameState))
      (Variables|/Game/Blueprints/BP_YGO_GameState.BP_YGO_GameState_C|SetCurrentBattleStep _gamestate "NewEnumerator1"))
    (:NewEnumerator4
      (CallFunction|OnMain2PhaseStart))
    (:NewEnumerator5
      (CallFunction|OnEndPhaseStart))))

(fn SwitchTurnPlayer
  (bind _players (Variables|Default|GetPlayers))
  (bind _output (Utilities|Array|Get(acopy) _players))
  (bind _playerstate (Variables|/Script/Engine.Controller|GetPlayerState _output))
  (bind _gamestate (CallFunction|GetGameState))
  (if (== _playerstate (Variables|/Game/Blueprints/BP_YGO_GameState.BP_YGO_GameState_C|GetCurrentTurnPlayer _gamestate))
    (bind _asbp_ygo_player_state (Utilities|Casting|CastToBP_YGO_PlayerState (Variables|/Script/Engine.Controller|GetPlayerState (Utilities|Array|Get(acopy) (Variables|Default|GetPlayers) 1))))
    (Variables|/Game/Blueprints/BP_YGO_GameState.BP_YGO_GameState_C|SetCurrentTurnPlayer _gamestate _asbp_ygo_player_state)
    (else
      (bind _asbp_ygo_player_state_2 (Utilities|Casting|CastToBP_YGO_PlayerState _playerstate))
      (Variables|/Game/Blueprints/BP_YGO_GameState.BP_YGO_GameState_C|SetCurrentTurnPlayer _gamestate _asbp_ygo_player_state_2))))

(fn StartGame
  (bind _gamestate (CallFunction|GetGameState))
  (bind _output_get (Variables|/Game/Blueprints/BP_YGO_GameState.BP_YGO_GameState_C|SetTurnCount _gamestate 1))
  (Variables|Default|SetremainNormalSummonCount 1)
  (CallFunction|OnTurnChanged (Variables|/Game/Blueprints/BP_YGO_GameState.BP_YGO_GameState_C|GetCurrentTurnPlayer _gamestate) _output_get)
  (CallFunction|EnterPhase "NewEnumerator0"))

(fn AdvancePhase
  (params (NextPhase :type E_TurnPhase%20Enum :default "NewEnumerator0"))
  (bind _gamestate (CallFunction|GetGameState))
  (switch Utilities|FlowControl|Switch|SwitchonE_TurnPhase (Variables|/Game/Blueprints/BP_YGO_GameState.BP_YGO_GameState_C|GetCurrentTurnPhase _gamestate)
    (:NewEnumerator0
      (LocalVariables|SetPhase "NewEnumerator1")
      (CallFunction|EnterPhase (LocalVariables|GetPhase) :!label _label))
    (:NewEnumerator1
      (LocalVariables|SetPhase "NewEnumerator2")
      (goto _label))
    (:NewEnumerator2
      (if (Variables|Default|GetisFirstTurn)
        (LocalVariables|SetPhase "NewEnumerator5")
        (goto _label)
        (elif (or (Utilities|Enum|Equal(Enum) NextPhase "NewEnumerator3") (Utilities|Enum|Equal(Enum) NextPhase "NewEnumerator5"))
          (LocalVariables|SetPhase NextPhase)
          (goto _label))))
    (:NewEnumerator3
      (LocalVariables|SetPhase "NewEnumerator4")
      (goto _label))
    (:NewEnumerator4
      (LocalVariables|SetPhase "NewEnumerator5")
      (goto _label))
    (:NewEnumerator5
      ;[0.15 0.15 0.15 0.5] after this, return;
      (Turn|EndTurn))))

(fn EndTurn
  (CallFunction|SwitchTurnPlayer)
  (bind _gamestate (CallFunction|GetGameState))
  (bind _result (Math|Integer|IncrementInt (Variables|/Game/Blueprints/BP_YGO_GameState.BP_YGO_GameState_C|GetTurnCount _gamestate))
    (:%20%20
      (Variables|Default|SetremainNormalSummonCount 1)
      (Variables|Default|SetisFirstTurn false)
      (CallFunction|OnTurnChanged (Variables|/Game/Blueprints/BP_YGO_GameState.BP_YGO_GameState_C|GetCurrentTurnPlayer _gamestate) _result)
      (CallFunction|EnterPhase "NewEnumerator0"))))

(fn ForceSetPhase
  (params (TurnPhase :type E_TurnPhase%20Enum :default "NewEnumerator0"))
  (CallFunction|EnterPhase TurnPhase))

(fn GetCurrentTurnPhase
  (bind _gamestate (CallFunction|GetGameState))
  (return (Variables|/Game/Blueprints/BP_YGO_GameState.BP_YGO_GameState_C|GetCurrentTurnPhase _gamestate)))

(fn GetCurrentBattleStep
  (bind _gamestate (CallFunction|GetGameState))
  (return (Variables|/Game/Blueprints/BP_YGO_GameState.BP_YGO_GameState_C|GetCurrentBattleStep _gamestate)))

(fn GetCurrentDamageStep
  (bind _gamestate (CallFunction|GetGameState))
  (return (Variables|/Game/Blueprints/BP_YGO_GameState.BP_YGO_GameState_C|GetCurrentDamageStep _gamestate)))

(fn GetCurrentTurnPlayer
  (bind _gamestate (CallFunction|GetGameState))
  (return (Variables|/Game/Blueprints/BP_YGO_GameState.BP_YGO_GameState_C|GetCurrentTurnPlayer _gamestate)))

(fn GetTurnCount
  (bind _gamestate (CallFunction|GetGameState))
  (return (Variables|/Game/Blueprints/BP_YGO_GameState.BP_YGO_GameState_C|GetTurnCount _gamestate)))

(fn IsPlayerTurn
  (params (PlayerController :type BP%20YGO%20Player%20Controller%20Object%20Reference))
  (bind _playerstate (Getters|GetCurrentTurnPlayer))
  (bind _asbp_ygo_player_state (Utilities|Casting|CastToBP_YGO_PlayerState (Variables|/Script/Engine.Controller|GetPlayerState PlayerController)))
  (return (== _playerstate _asbp_ygo_player_state)))

(fn CanNormalSummon
  (bind _turnphase (Getters|GetCurrentTurnPhase))
  (if (or (Utilities|Enum|Equal(Enum) _turnphase "NewEnumerator2") (Utilities|Enum|Equal(Enum) _turnphase "NewEnumerator4"))
    (return (> (Variables|Default|GetremainNormalSummonCount) 0))
    (else
      (return false))))

(fn ConsumeNormalSummon
  (Math|Integer|DecrementInt (Variables|Default|GetremainNormalSummonCount)))