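; Replicated card actor for a card game with face-up/down attack and defense positions.
; Looks up CardId in a data table to set the atlas index on its dynamic face material, refreshed by OnReps.
; StartMoving hands the card between field positions on authority and prepares an eased move for UpdateMovement, which nothing here calls.
; Tick drives simple moves and flips; position changes snap (animation TODO), and debug mouse handlers are never bound.
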(event Custom|OnCardClicked
  (params (TouchedActor :type Actor%20Object%20Reference) (ButtonPressed :type Key%20Structure :default "None"))
  (Development|PrintText (Utilities|Text|FormatText "OnCard Clicked instanceID {0} touchedActor {1} button {2}" (Variables|CardStatus|GetinstanceId) TouchedActor (Class|KismetInputLibrary|KeyGetDisplayName ButtonPressed true))))

(event Custom|OnBeginCursorOver_Event
  (params (TouchedActor :type Actor%20Object%20Reference))
  (Development|PrintText (Utilities|Text|FormatText "OnCard BeginCursorOver instanceID {0} touchedActor{1}" (Variables|CardStatus|GetinstanceId) TouchedActor)))

(event Custom|OnEndCursorOver_Event
  (params (TouchedActor :type Actor%20Object%20Reference))
  (Development|PrintText (Utilities|Text|FormatText "OnCard EndCursorOver instanceID {0} touchedActor{1}" (Variables|CardStatus|GetinstanceId) TouchedActor)))

(event EventBeginPlay
  (bind _returnvalue (Rendering|Material|CreateDynamicMaterialInstance (Variables|Default|GetPlane_Face) 0 "/Game/Material/M_CardAtlas_Inst.M_CardAtlas_Inst" "None" :!class /Script/Engine.PrimitiveComponent))
  (bind _output_get (Variables|Default|SetFaceMaterial _returnvalue))
  (Rendering|Material|SetMaterial (Variables|Default|GetPlane_Face) 0 _output_get))

(event Collision|EventActorBeginOverlap
  (params (OtherActor :type Actor%20Object%20Reference)))

(event EventTick
  (params (DeltaSeconds :type Float%20%28single-precision%29))
  (if (Variables|Animation|GetisAnimating)
    (Update|UpdateAnimation DeltaSeconds)))

(fn ConstructionScript)

(fn Setup
  (params (cardId :type Integer))
  (bind _facematerial (Variables|Default|GetFaceMaterial))
  ;[0.15 0.15 0.15 0.5] if cardId != -1 ? find in table : use default sprite index
  (if (!= cardId -1)
    (bind _returnvalue (Utilities|GetDataTableRow (Variables|Default|GetssIndexTable) (Utilities|String|StringToName (Utilities|String|ToString(Integer) cardId)))
      (:then
        (Rendering|Material|SetScalarParameterValue _facematerial "Index" (Math|Conversions|ToFloat(Integer) (Utilities|Struct|BreakSTR_SpriteSheetIndex _returnvalue)) :!class /Script/Engine.MaterialInstanceDynamic))
      (:RowNotFound
        (Development|PrintText (Utilities|Text|FormatText "Failed to find card sprite sheet index of {0}" cardId))))
    (else
      (bind _output_get (LocalVariables|SetactualUsingIndex 0))
      (Rendering|Material|SetScalarParameterValue _facematerial "Index" (Math|Conversions|ToFloat(Integer) _output_get) :!class /Script/Engine.MaterialInstanceDynamic))))

(fn SetPositionObjectRef
  (params (posObject :type BP%20Field%20Position%20Object%20Reference))
  (Variables|Default|SetcurrentFieldPosition posObject))

(fn StartMoving
  (params (TargetPosition :type BP%20Field%20Position%20Object%20Reference) (duration :type Float%20%28double-precision%29))
  (bind _currentfieldposition (Variables|Default|GetcurrentFieldPosition))
  (if (Ability|HasAuthority)
    (Utilities|IsValid _currentfieldposition
      (:Is%20Valid
        (Default|RemoveCard _currentfieldposition self))
      (:Is%20Not%20Valid
        _))
    (Default|AddCard TargetPosition self)
    (Variables|Default|SetPendingFP TargetPosition)
    (Variables|Animation|SetMoveDuration duration)
    (Variables|Animation|SetMoveProgress 0.0)
    (Variables|Animation|SetStartLocation (Transformation|GetActorLocation))
    (Variables|Animation|SetStartRotation (Transformation|GetActorRotation))
    (bind _worldlocation (Default|GetCardSlotLocation TargetPosition))
    (Variables|Animation|SetTargetLocation _worldlocation)
    (bind _rotator (CallFunction|GetCardDesiredRelativeRotation))
    (Variables|Animation|SetTargetRotation (Math|Rotator|CombineRotators _rotator (Transformation|GetActorRotation TargetPosition)))
    (Variables|Animation|SetisMoving true)))

(fn GetCardDesiredRelativeRotation
  (switch Utilities|FlowControl|Switch|SwitchonE_CardPosition (Variables|CardStatus|GetcurrentCardPosition)
    (:NewEnumerator0
      (LocalVariables|SetyRot 0.0)
      (LocalVariables|SetzRot 9e+01))
    (:NewEnumerator1
      (LocalVariables|SetyRot 0.0)
      (LocalVariables|SetzRot 1.8e+02))
    (:NewEnumerator2
      (LocalVariables|SetyRot 1.8e+02)
      (LocalVariables|SetzRot 9e+01))
    (:NewEnumerator3
      (LocalVariables|SetyRot 1.8e+02)
      (LocalVariables|SetzRot 1.8e+02)))
  (return (Math|Rotator|MakeRotator 0.0 (LocalVariables|GetyRot) (LocalVariables|GetzRot))))

(fn UpdateMovement
  (params (deltaTime :type Float%20%28double-precision%29))
  (bind _moveduration (Variables|Animation|GetMoveDuration))
  (bind _pendingfp (Variables|Default|GetPendingFP))
  (bind _output_get (Variables|Animation|SetMoveProgress (+ (Variables|Animation|GetMoveProgress) deltaTime)))
  (if (>= _output_get _moveduration)
    ;[0.15 0.15 0.15 0.5] End moving
    (Variables|Animation|SetMoveProgress _moveduration)
    (Variables|Animation|SetisMoving false)
    (Utilities|IsValid _pendingfp
      (:Is%20Valid
        (Default|OnCardMoveEnd _pendingfp self)))
    (else
      ;[0.15 0.15 0.15 0.5] Move
      (bind _output_get_2 (LocalVariables|Setalpha (Class|KismetMathLibrary|FInterpEaseinOut 0.0 1.0 (Math|Float|SafeDivide (Variables|Animation|GetMoveProgress) (Variables|Animation|GetMoveDuration)) 2.0)))
      (Transformation|SetActorLocationAndRotation (Math|Vector|Lerp(Vector) (Variables|Animation|GetStartLocation) (Variables|Animation|GetTargetLocation) _output_get_2) (Math|Rotator|Lerp(Rotator) (Variables|Animation|GetStartRotation) (Variables|Animation|GetTargetRotation) _output_get_2 true)))))

(fn InitializeCard
  (params (cardId :type Integer) (owner :type BP%20YGO%20Player%20Controller%20Object%20Reference))
  (Variables|CardStatus|SetcardId cardId)
  (Variables|CardStatus|SetownerController owner)
  (Update|UpdateCardAppearance))

(fn SetFaceUp
  (params (FaceUp :type Boolean) (Animate :type Boolean))
  (if (not (== FaceUp (Variables|CardStatus|GetisFacingUp)))
    (Variables|CardStatus|SetisFacingUp FaceUp)
    (if (and (not (Variables|Animation|GetisFlipping)) Animate)
      (Variables|Animation|SetisFlipping true)
      (Variables|Animation|SetisAnimating true)
      (Variables|Animation|SetflipTargetFaceUp FaceUp)
      (Variables|Animation|SetflipProgress 0.0)
      (else
        (Update|UpdateCardAppearance)))))

(fn SetCardPosition
  (params (NewPosition :type E_CardPosition%20Enum :default "NewEnumerator0") (Animate :type Boolean))
  (bind _output_get (Variables|CardStatus|SetcurrentCardPosition NewPosition))
  (switch Utilities|FlowControl|Switch|SwitchonE_CardPosition _output_get
    (:NewEnumerator0
      (LocalVariables|SetyRot 0.0)
      (LocalVariables|SetzRot 9e+01)
      (Variables|CardStatus|SetisFacingUp true :!label _label))
    (:NewEnumerator1
      (LocalVariables|SetyRot 0.0)
      (LocalVariables|SetzRot 1.8e+02)
      (goto _label))
    (:NewEnumerator2
      (LocalVariables|SetyRot 1.8e+02)
      (LocalVariables|SetzRot 9e+01)
      (Variables|CardStatus|SetisFacingUp false :!label _label_2))
    (:NewEnumerator3
      (LocalVariables|SetyRot 1.8e+02)
      (LocalVariables|SetzRot 1.8e+02)
      (goto _label_2)))
  (if Animate
    _
    (else
      _))
  ;[0.15 0.15 0.15 0.5] TODO animate
  (Transformation|SetActorRelativeRotation (Math|Rotator|MakeRotator 0.0 (LocalVariables|GetyRot) (LocalVariables|GetzRot)))
  (Update|UpdateCardAppearance))

(fn SetCardZone
  (params (cardZone :type E_CardZone%20Enum :default "NewEnumerator0"))
  (Variables|CardStatus|SetcurrentZone cardZone))

(fn MovetoLocation
  (params (TargetLocation :type Vector) (Animate :type Boolean))
  (if Animate
    (Variables|Animation|SetTargetLocation TargetLocation)
    (Variables|Animation|SetisMoving true)
    (Variables|Animation|SetisAnimating true)
    (else
      (Transformation|SetActorLocation TargetLocation false false))))

(fn IsFaceUp
  (return (Variables|CardStatus|GetisFacingUp)))

(fn GetCardPositionObj
  (return (Variables|Default|GetcurrentFieldPosition)))

(fn GetOwnerController
  (return (Variables|CardStatus|GetownerController)))

(fn GetInstanceId
  (return (Variables|CardStatus|GetinstanceId)))

(fn OnRepIsFacingUp
  (Update|UpdateCardAppearance))

(fn OnRepCurrentCardPosition
  (Card|SetCardPosition (Variables|CardStatus|GetcurrentCardPosition) false))

(fn GetCardZone
  (return (Variables|CardStatus|GetcurrentZone)))

(fn UpdateCardAppearance
  (bind _facematerial (Variables|Default|GetFaceMaterial))
  (bind _cardid (Variables|CardStatus|GetcardId))
  ;[0.15 0.15 0.15 0.5] if cardId != -1 ? find in table : use default sprite index
  (if (!= _cardid -1)
    (bind _returnvalue (Utilities|GetDataTableRow (Variables|Default|GetssIndexTable) (Utilities|String|StringToName (Utilities|String|ToString(Integer) _cardid)))
      (:then
        (Rendering|Material|SetScalarParameterValue _facematerial "Index" (Math|Conversions|ToFloat(Integer) (Utilities|Struct|BreakSTR_SpriteSheetIndex _returnvalue)) :!class /Script/Engine.MaterialInstanceDynamic))
      (:RowNotFound
        (Development|PrintText (Utilities|Text|FormatText "Failed to find card sprite sheet index of {0}" _cardid))))
    (else
      (bind _output_get (LocalVariables|SetActualUsingIndex 0))
      (Rendering|Material|SetScalarParameterValue _facematerial "Index" (Math|Conversions|ToFloat(Integer) _output_get) :!class /Script/Engine.MaterialInstanceDynamic))))

(fn UpdateAnimation
  (params (deltaTime :type Float%20%28double-precision%29))
  (if (Variables|Animation|GetisMoving)
    (bind _output_get (LocalVariables|SetcurrentLocation (Transformation|GetActorLocation)))
    (bind _output_get_2 (LocalVariables|Setdirection (- (Variables|Animation|GetTargetLocation) _output_get)))
    (LocalVariables|Setdistance (Math|Vector|VectorLength _output_get_2))
    (if (< (LocalVariables|Getdistance) 1.0)
      (Transformation|SetActorLocation (Variables|Animation|GetTargetLocation) false false)
      (Variables|Animation|SetisMoving false)
      (else
        (Transformation|SetActorLocation (+ (LocalVariables|GetcurrentLocation) (* (Math|Vector|Normalize (LocalVariables|Getdirection)) (Variables|Animation|GetmoveAnimationSpeed) deltaTime)) false false))))
  (if (Variables|Animation|GetisFlipping)
    (bind _output_get_3 (Variables|Animation|SetflipProgress (+ (* (Variables|Animation|GetflipAnimationSpeed) deltaTime) (Variables|Animation|GetflipProgress))))
    (if (>= _output_get_3 1.0)
      (Variables|Animation|SetflipProgress 1.0)
      (Variables|Animation|SetisFlipping false)
      (Update|UpdateCardAppearance)
      (else
        (if (>= (Variables|Animation|GetflipProgress) 0.5)
          (Update|UpdateCardAppearance))
        (bind _output_get_4 (LocalVariables|SetcurrentRotation (Transformation|GetActorRotation)))
        (Transformation|SetActorRotation (Math|Rotator|MakeRotator (.Roll (Math|Rotator|BreakRotator _output_get_4)) (Math|Float|Lerp 0.0 1.8e+02 (Variables|Animation|GetflipProgress)) (.Yaw (Math|Rotator|BreakRotator _output_get_4))))))))

(fn OnRepCardId
  (Update|UpdateCardAppearance))