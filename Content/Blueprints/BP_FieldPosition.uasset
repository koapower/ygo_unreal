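; Field slot actor for a card game that holds an ordered stack of cards at one zone, identified by PositionId.
; AddCard registers a card, and OnCardMoveEnd attaches it and restacks all cards by thickness, applying each card's desired rotation.
; GetCardSlotLocation gives the world point above the stack, while removal functions detach cards.
; IsFull limits monster, spell/trap and field zones to one card, leaves piles and hand unlimited, and treats undefined as full.
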(event EventBeginPlay)

(event Collision|EventActorBeginOverlap
  (params (OtherActor :type Actor%20Object%20Reference)))

(event EventTick
  (params (DeltaSeconds :type Float%20%28single-precision%29)))

(fn ConstructionScript)

(fn AddCard
  (params (card :type BP%20Card%20Object%20Reference))
  (Utilities|Array|Add (Variables|Default|GetCardArray) card))

(fn OnCardMoveEnd
  (params (card :type BP%20Card%20Object%20Reference))
  (Transformation|AttachComponentToComponent card (Variables|Default|GetDefaultSceneRoot) "None" "SnapToTarget" "SnapToTarget" "KeepWorld" true)
  (CallFunction|RefreshCards))

(fn RefreshCards
  (for (_array_element _array_index) (Variables|Default|GetCardArray)
    ;[0.15 0.15 0.15 0.5] Position
    (Transformation|SetActorRelativeLocation _array_element (+ (Math|Vector|MakeVector 0.0 0.0 (* (+ _array_index 1) (Variables|Default|GetCardThickness))) (Variables|Default|GetpositionOffset)))
    ;[0.15 0.15 0.15 0.5] Rotation
    (bind _rotator (Default|GetCardDesiredRelativeRotation _array_element))
    (Transformation|SetActorRelativeRotation _array_element _rotator)))

(fn RemoveCard
  (params (card :type BP%20Card%20Object%20Reference))
  (bind _returnvalue (Utilities|Array|RemoveItem (Variables|Default|GetCardArray) card))
  (if _returnvalue
    (Transformation|DetachFromActor card "KeepWorld" "KeepWorld" "KeepWorld")
    (CallFunction|RefreshCards)
    (return true)
    (else
      (return false))))

(fn GetTopCard
  (bind _cardarray (Variables|Default|GetCardArray))
  (bind _returnvalue (Utilities|Array|Length _cardarray))
  (if (> _returnvalue 0)
    (return (Utilities|Array|Get(acopy) _cardarray (- _returnvalue 1)))))

(fn GetCardSlotLocation
  (return (+ (Math|Vector|MakeVector 0.0 0.0 (* (+ (Utilities|Array|Length (Variables|Default|GetCardArray)) 1) (Variables|Default|GetCardThickness))) (+ (Transformation|GetActorLocation) (Variables|Default|GetpositionOffset)))))

(fn RemoveAllCards
  (bind _cardarray (Variables|Default|GetCardArray))
  (for _array_element _cardarray
    (Transformation|DetachFromActor _array_element "KeepWorld" "KeepWorld" "KeepWorld"))
  (Utilities|Array|Clear _cardarray)
  (CallFunction|RefreshCards))

(fn IsFull
  (switch Utilities|FlowControl|Switch|SwitchonE_FieldPosition (Variables|Default|GetPositionId)
    (:NewEnumerator30
      (return true))
    (:NewEnumerator0
      _)
    (:NewEnumerator1
      _)
    (:NewEnumerator2
      _)
    (:NewEnumerator3
      _)
    (:NewEnumerator4
      (return (> (Utilities|Array|Length (Variables|Default|GetCardArray)) 0)))
    (:NewEnumerator5
      (return (> (Utilities|Array|Length (Variables|Default|GetCardArray)) 0)))
    (:NewEnumerator6
      (return (> (Utilities|Array|Length (Variables|Default|GetCardArray)) 0)))
    (:NewEnumerator7
      (return (> (Utilities|Array|Length (Variables|Default|GetCardArray)) 0)))
    (:NewEnumerator8
      (return (> (Utilities|Array|Length (Variables|Default|GetCardArray)) 0)))
    (:NewEnumerator9
      (return (> (Utilities|Array|Length (Variables|Default|GetCardArray)) 0)))
    (:NewEnumerator10
      (return (> (Utilities|Array|Length (Variables|Default|GetCardArray)) 0)))
    (:NewEnumerator11
      (return (> (Utilities|Array|Length (Variables|Default|GetCardArray)) 0)))
    (:NewEnumerator12
      (return (> (Utilities|Array|Length (Variables|Default|GetCardArray)) 0)))
    (:NewEnumerator13
      (return (> (Utilities|Array|Length (Variables|Default|GetCardArray)) 0)))
    (:NewEnumerator14
      (return (> (Utilities|Array|Length (Variables|Default|GetCardArray)) 0)))
    (:NewEnumerator31
      _))
  (return false))