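; Turn manager for a two-player card game, tracking the current player, phase and turn count.
; AdvancePhase steps through Draw, Standby, Main 1, Battle, Main 2 and End; Main 1 skips to End on turn one, otherwise taking the requested Battle or End phase.
; Leaving End calls EndTurn, which passes play to the next player at Draw.
; Dispatchers announce turn and phase changes, while CanPerformAction checks player and phase.
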(event Custom|OnTurnChanged
  (params (NewTurnPlayerId :type Integer) (Phase :type E_TurnPhase%20Enum :default "NewEnumerator0")))

(event Custom|OnPhaseChanged
  (params (NewPhase :type E_TurnPhase%20Enum :default "NewEnumerator0")))

(fn InitializeTurn
  (params (StartingPlayerID :type Integer))
  (bind _playerids (Variables|Default|GetPlayerIds))
  (Utilities|Array|Clear _playerids)
  (Utilities|Array|Add _playerids 0)
  (Utilities|Array|Add _playerids 1)
  (if (== StartingPlayerID 0)
    (Variables|Turn|SetCurrentTurnPlayerId 0)
    (else
      (Variables|Turn|SetCurrentTurnPlayerId 1)))
  (Variables|Turn|SetCurrentPhase "NewEnumerator0")
  (Variables|Turn|SetTurnCount 1)
  (CallFunction|OnTurnChanged (Variables|Turn|GetCurrentTurnPlayerId) (Variables|Turn|GetCurrentPhase)))

(fn AdvancePhase
  (params (NextPhase :type E_TurnPhase%20Enum :default "NewEnumerator0"))
  (switch Utilities|FlowControl|Switch|SwitchonE_TurnPhase (Variables|Turn|GetCurrentPhase)
    (:NewEnumerator0
      (Variables|Turn|SetCurrentPhase "NewEnumerator1")
      (CallFunction|OnPhaseChanged (Variables|Turn|GetCurrentPhase) :!label _label))
    (:NewEnumerator1
      (Variables|Turn|SetCurrentPhase "NewEnumerator2")
      (goto _label))
    (:NewEnumerator2
      (if (== (Variables|Turn|GetTurnCount) 1)
        (Variables|Turn|SetCurrentPhase "NewEnumerator5")
        (goto _label)
        (elif (or (Utilities|Enum|Equal(Enum) NextPhase "NewEnumerator3") (Utilities|Enum|Equal(Enum) NextPhase "NewEnumerator5"))
          (Variables|Turn|SetCurrentPhase NextPhase)
          (goto _label))))
    (:NewEnumerator3
      (Variables|Turn|SetCurrentPhase "NewEnumerator4")
      (goto _label))
    (:NewEnumerator4
      (Variables|Turn|SetCurrentPhase "NewEnumerator5")
      (goto _label))
    (:NewEnumerator5
      ;[0.15 0.15 0.15 0.5] after this, return;
      (Turn|EndTurn))))

(fn EndTurn
  (bind _output_get (Variables|Default|SetCurrentPlayerIndex (Math|Integer|%(Integer) (+ (Variables|Turn|GetCurrentTurnPlayerId) 1) (Utilities|Array|Length (Variables|Default|GetPlayerIds)))))
  (Variables|Turn|SetCurrentTurnPlayerId (Utilities|Array|Get(acopy) (Variables|Default|GetPlayerIds) _output_get))
  (Variables|Turn|SetCurrentPhase "NewEnumerator0")
  (Math|Integer|IncrementInt (Variables|Turn|GetTurnCount)
    (:%20%20
      (CallFunction|OnTurnChanged (Variables|Turn|GetCurrentTurnPlayerId) (Variables|Turn|GetCurrentPhase)))))

(fn IsPlayerTurn
  (params (PlayerId :type Integer))
  (return (== (Variables|Turn|GetCurrentTurnPlayerId) PlayerId)))

(fn CanPerformAction
  (params (PlayerId :type Integer) (RequiredPhase :type E_TurnPhase%20Enum :default "NewEnumerator0"))
  (bind _isplayerturn (Turn|IsPlayerTurn PlayerId))
  (return (and _isplayerturn (Utilities|Enum|Equal(Enum) (Variables|Turn|GetCurrentPhase) RequiredPhase))))