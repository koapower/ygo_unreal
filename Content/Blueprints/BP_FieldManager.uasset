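; Field manager for a two-player card game that spawns cards and manages their placement on each player's board positions.
; Positions are looked up by ID in per-player arrays, then cards move there over time or are removed.
; SpawnCard is authority-only and ignores its Location input; placement rejects full slots and skips hand positions.
; MoveCardToPos always targets player 0, and IsPositionAvailable is a stub returning false.
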(event EventBeginPlay)

(event Collision|EventActorBeginOverlap
  (params (OtherActor :type Actor%20Object%20Reference)))

(event EventTick
  (params (DeltaSeconds :type Float%20%28single-precision%29)))

(fn ConstructionScript)

(fn SpawnCard
  (params (cardId :type Integer) (Location :type Vector))
  (if (Ability|HasAuthority)
    (bind _returnvalue (Game|SpawnActorfromClass "/Game/Blueprints/BP_Card.BP_Card_C" (Math|Transform|MakeTransform "0.000000,0.000000,1.000000" "180.000000,0.000000,0.000000") "Undefined" "MultiplyWithRoot" 0 0))
    (Default|Setup _returnvalue cardId)
    (return _returnvalue)))

(fn MoveCardtoPos
  (params (card :type BP%20Card%20Object%20Reference) (fieldPos :type E_FieldPosition%20Enum :default "NewEnumerator0"))
  (bind _posobject (Field|GetPositionObject 0 fieldPos))
  (Utilities|IsValid _posobject
    (:Is%20Valid
      (Default|StartMoving card _posobject 0.5))
    (:Is%20Not%20Valid
      (Development|PrintText (Utilities|Text|FormatText "Failed to get field position object for {0}" (Utilities|String|EnumtoString fieldPos))))))

(fn GetPositionObject
  (params (PlayerId :type Integer) (Pos :type E_FieldPosition%20Enum :default "NewEnumerator30"))
  (if (== PlayerId 0)
    (LocalVariables|SettargetPositionArray (Variables|Default|GetPositions_0))
    (else
      (LocalVariables|SettargetPositionArray (Variables|Default|GetPositions_1))))
  (bind _array_element (Utilities|Array|ForEachLoopwithBreak (LocalVariables|GettargetPositionArray))
    (:LoopBody
      (if (Utilities|Enum|Equal(Enum) Pos (Variables|/Game/Blueprints/BP_FieldPosition.BP_FieldPosition_C|GetPositionId _array_element))
        (return _array_element)))))

(fn InitializeField
  (for _array_element (Variables|Default|GetPositions_0)
    (Default|RemoveAllCards _array_element))
  (for _array_element_2 (Variables|Default|GetPositions_1)
    (Default|RemoveAllCards _array_element_2)))

(fn PlaceCardonField
  (params (PlayerId :type Integer) (Card :type BP%20Card%20Object%20Reference) (FieldPosition :type E_FieldPosition%20Enum :default "NewEnumerator30"))
  (if (Utilities|Enum|Equal(Enum) FieldPosition "NewEnumerator31")
    ;[0.15 0.15 0.15 0.5] HandPosition will be dealt separately
    (return true)
    (else
      (bind _posobject (Field|GetPositionObject PlayerId FieldPosition))
      (Utilities|IsValid _posobject
        (:Is%20Valid
          (bind _isfull (Default|IsFull _posobject))
          (if _isfull
            (return false)
            (else
              (Default|StartMoving Card _posobject 0.5)
              (return true))))
        (:Is%20Not%20Valid
          (Development|PrintText (Utilities|Text|FormatText "Failed to find position object for playerId {0} position {1}!" PlayerId (Utilities|String|EnumtoString FieldPosition)))
          (return false))))))

(fn RemoveCardfromField
  (params (card :type BP%20Card%20Object%20Reference) (PlayerId :type Integer) (FieldPosition :type E_FieldPosition%20Enum :default "NewEnumerator30"))
  (bind _posobject (Field|GetPositionObject PlayerId FieldPosition))
  (Utilities|IsValid _posobject
    (:Is%20Valid
      (bind _successful (Default|RemoveCard _posobject card))
      (return _successful))
    (:Is%20Not%20Valid
      (return false))))

(fn IsPositionAvailable
  (params (PlayerId :type Integer) (FieldPosition :type E_FieldPosition%20Enum :default "NewEnumerator30"))
  (return false))